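; AI controller for BP_CharNPC_Enemy that moves the enemy toward whoever it perceives or is damaged by.
; Perception updates pass an IsLife check and target only BP_CharPlayer, while Damage_Perception targets the damage dealer.
; When MoveToActor reports Already at Goal, ShotingValid guards creation of a single looping timer, whose event binding is not shown.
; Shot spawns an Arrow_Bullet_Enemy at the enemy's ArrowWeapon transform.
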(event OnTargetPerceptionUpdated(AIPerception)
  (params (Actor :type Actor%20Object%20Reference) (Stimulus :type AI%20Stimulus%20Structure))
  (if (Utilities|IsLife)
    (bind _asbp_char_player (Utilities|Casting|CastToBP_CharPlayer Actor))
    (bind _returnvalue (AI|Navigation|MovetoActor _asbp_char_player 5e+01 true true true 0))
    (switch Utilities|FlowControl|Switch|SwitchonEPathFollowingRequestResult _returnvalue
      (:AlreadyAtGoal
        (bind _returnvalue_2 (CallFunction|ShotingValid))
        (if _returnvalue_2
          (bind _returnvalue_3 (Utilities|Time|SetTimerbyEvent (EventDispatchers|CreateEvent :!event Shot) 2.0 true))
          (Variables|Default|SetShotingEvent _returnvalue_3))))))

(event Custom|Damage_Perception
  (params (Damage_Dealer :type Actor%20Object%20Reference))
  (bind _returnvalue (AI|Navigation|MovetoActor Damage_Dealer 5e+01 true true true 0))
  (switch Utilities|FlowControl|Switch|SwitchonEPathFollowingRequestResult _returnvalue
    (:AlreadyAtGoal
      (bind _returnvalue_2 (CallFunction|ShotingValid))
      (if _returnvalue_2
        (bind _returnvalue_3 (Utilities|Time|SetTimerbyEvent (EventDispatchers|CreateEvent :!event Shot) 2.0 true))
        (Variables|Default|SetShotingEvent _returnvalue_3)))))

(event EventBeginPlay
  (bind _asbp_char_npc_enemy (Utilities|Casting|CastToBP_CharNPC_Enemy (Pawn|GetControlledPawn)))
  (Variables|Default|SetTargetNPC _asbp_char_npc_enemy))

(event EventTick
  (params (DeltaSeconds :type Float%20%28single-precision%29)))

(fn ConstructionScript)

(fn Shot
  (bind _targetnpc (Variables|Default|GetTargetNPC))
  (Game|SpawnActorfromClass "/Game/Blueprints/Magik(Weapon)/EnemyBullet/Arrow_Bullet_Enemy.Arrow_Bullet_Enemy_C" (Transformation|GetWorldTransform (Variables|/Game/Blueprints/NPC/BP_CharNPC_Enemy.BP_CharNPC_Enemy_C|GetArrow_weapon _targetnpc)) "AlwaysSpawn" _targetnpc 0))

(fn ShotingValid
  (return (not (Utilities|Time|IsValidTimerHandle (Variables|Default|GetShotingEvent)))))
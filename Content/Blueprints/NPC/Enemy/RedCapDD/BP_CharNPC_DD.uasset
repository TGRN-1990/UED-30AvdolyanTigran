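; BP_CharNPC_DD is the Blueprint for the RedCapDD enemy NPC character, connecting stat updates to death handling and the health widget.
; When a stats update reports death, it fires DeadActor, which calls DeadNPC.
; Otherwise it casts the WidgetNPCHealt user widget to BP_widjet_NPC_bar and assigns itself as that bar's NPC.
; Tick and construction only defer to the parent class.
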(event Custom|DeadActor
  (CallFunction|DeadNPC))

(event EventBeginPlay
  (|CallParentFunction) ; This node is disabled and will not be called.\nDrag off pins to build functionality.
)

(event Collision|EventActorBeginOverlap
  (params (OtherActor :type Actor%20Object%20Reference))
  (|CallParentFunction OtherActor) ; This node is disabled and will not be called.\nDrag off pins to build functionality.
)

(event EventTick
  (params (DeltaSeconds :type Float%20%28single-precision%29))
  (|CallParentFunction DeltaSeconds))

(fn ConstructionScript
  (|CallParentFunction))

(fn BPonStatsUpdated
  (params (IsDead :type Boolean) (ItsDamage :type Boolean) (CurrentHP :type Integer) (CurrentEP :type Integer))
  (if IsDead
    (CallFunction|DeadActor)
    (else
      (bind _asbp_widjet_npc_bar (Utilities|Casting|CastToBP_widjet_NPC_bar (UserInterface|GetUserWidgetObject (Variables|Default|GetWidget_NPC_healt))))
      (Variables|/Game/Blueprints/BP_HUD/BP_Widjet/BP_widjet_NPC_bar.BP_widjet_NPC_bar_C|SetNPC _asbp_widjet_npc_bar self))))
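; Tiny enemy NPC character that trades damage with the player on contact.
; Capsule overlap with the player stores them, sets Battle and applies equal damage both ways, which Tick repeats every frame with no reset of the flag.
; The stats-updated callback points the health bar widget at this NPC or, on death, triggers an alarm sound and delayed destruction.
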(event OnComponentBeginOverlap(Capsule)
  (params (OverlappedComponent :type Primitive%20Component%20Object%20Reference) (OtherActor :type Actor%20Object%20Reference) (OtherComp :type Primitive%20Component%20Object%20Reference) (OtherBodyIndex :type Integer) (bFromSweep :type Boolean) (SweepResult :type Hit%20Result%20Structure%20%28by%20ref%29))
  (bind _asbp_char_player (Utilities|Casting|CastToBP_CharPlayer OtherActor))
  (Variables|Default|SetPlayerCautch _asbp_char_player)
  (Variables|Default|Setbattle true)
  (Game|Damage|ApplyDamage (Variables|Default|GetPlayerCautch) 4e+01 0 self "/Game/Blueprints/Object/BP_DamageTypeObject.BP_DamageTypeObject_C")
  (Game|Damage|ApplyDamage self 4e+01 0 (Variables|Default|GetPlayerCautch) "/Game/Blueprints/Object/BP_DamageTypeObject.BP_DamageTypeObject_C"))

(event Custom|DeadActor
  (if true
    (Audio|SpawnSound2D "/Game/Retro_8Bit_Sounds/Alarms_Sirens/Wavs/retro_alarm_siren_loop_12.retro_alarm_siren_loop_12" 1.0 1.0 0.0 0)
    (Utilities|FlowControl|Delay 1.0)
    (Actor|DestroyActor)))

(event EventBeginPlay
  (|CallParentFunction) ; This node is disabled and will not be called.\nDrag off pins to build functionality.
)

(event Collision|EventActorBeginOverlap
  (params (OtherActor :type Actor%20Object%20Reference))
  (|CallParentFunction OtherActor) ; This node is disabled and will not be called.\nDrag off pins to build functionality.
)

(event EventTick
  (params (DeltaSeconds :type Float%20%28single-precision%29))
  (|CallParentFunction DeltaSeconds)
  (if (Variables|Default|Getbattle)
    (Game|Damage|ApplyDamage (Variables|Default|GetPlayerCautch) 4e+01 0 self "/Game/Blueprints/Object/BP_DamageTypeObject.BP_DamageTypeObject_C")
    (Game|Damage|ApplyDamage self 4e+01 0 (Variables|Default|GetPlayerCautch) "/Game/Blueprints/Object/BP_DamageTypeObject.BP_DamageTypeObject_C")))

(fn ConstructionScript
  (|CallParentFunction))

(fn BPonStatsUpdated
  (params (IsDead :type Boolean) (ItsDamage :type Boolean) (CurrentHP :type Integer) (CurrentEP :type Integer))
  (if IsDead
    (CallFunction|DeadActor)
    (else
      (bind _asbp_widjet_npc_bar (Utilities|Casting|CastToBP_widjet_NPC_bar (UserInterface|GetUserWidgetObject (Variables|Default|GetWidget_NPC_healt))))
      (Variables|/Game/Blueprints/BP_HUD/BP_Widjet/BP_widjet_NPC_bar.BP_widjet_NPC_bar_C|SetNPC _asbp_widjet_npc_bar self))))
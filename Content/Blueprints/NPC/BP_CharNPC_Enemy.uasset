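; Enemy NPC character that takes bullet and hitscan damage and displays a health widget.
; Capsule overlaps with bullets send damage to BPCharStats and report the shooter to the BP_AI_Enemy controller's damage perception.
; HitscanDamage only applies damage to the stats, without alerting the AI.
; Tick turns the health widget toward the player pawn, using only X and Y positions for the look-at.
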(event OnComponentBeginOverlap(Capsule)
  (params (OverlappedComponent :type Primitive%20Component%20Object%20Reference) (OtherActor :type Actor%20Object%20Reference) (OtherComp :type Primitive%20Component%20Object%20Reference) (OtherBodyIndex :type Integer) (bFromSweep :type Boolean) (SweepResult :type Hit%20Result%20Structure%20%28by%20ref%29))
  (CallFunction|BulletDamage OtherActor))

(event EventBeginPlay
  (|CallParentFunction)
  (bind _asbp_ai_enemy (Utilities|Casting|CastToBP_AI_Enemy (AI|GetAIController self)))
  (Variables|Default|SetAiControll _asbp_ai_enemy))

(event Collision|EventActorBeginOverlap
  (params (OtherActor :type Actor%20Object%20Reference))
  (|CallParentFunction OtherActor) ; This node is disabled and will not be called.\nDrag off pins to build functionality.
)

(event EventTick
  (params (DeltaSeconds :type Float%20%28single-precision%29))
  (bind _returnvalue (Game|Player|GetPlayerPawn 0))
  (bind _widget_npc_healt (Variables|Default|GetWidget_NPC_healt))
  (bind _returnvalue_2 (Transformation|GetActorLocation _returnvalue))
  (bind _returnvalue_3 (Transformation|GetWorldLocation _widget_npc_healt))
  (|CallParentFunction DeltaSeconds)
  (Transformation|SetWorldRotation _widget_npc_healt (Math|Rotator|FindLookatRotation (Math|Vector|MakeVector (.x _returnvalue_3) (.y _returnvalue_3) 0.0) (Math|Vector|MakeVector (.x _returnvalue_2) (.y _returnvalue_2) 0.0)) false false))

(fn ConstructionScript
  (|CallParentFunction))

(fn BulletDamage
  (params (Object :type Object%20Object%20Reference))
  (bind _asbp_bullet_base (Utilities|Casting|CastToBP_Bullet_Base Object))
  (bind _damage (Class|BPIWeapon|DamageDealer(Message) _asbp_bullet_base))
  (Default|ReceiveDamage (Variables|Default|GetBP_Char_Stats) _damage)
  (bind _asbp_ai_enemy (Utilities|Casting|CastToBP_AI_Enemy (AI|GetAIController self)))
  (Default|DamagePerception _asbp_ai_enemy (Variables|/Game/Blueprints/Magik(Weapon)/BP_Bullet_Base.BP_Bullet_Base_C|GetOwnerShoot _asbp_bullet_base)))

(fn HitscanDamage
  (params (Damage :type Integer))
  (Default|ReceiveDamage (Variables|Default|GetBP_Char_Stats) Damage))
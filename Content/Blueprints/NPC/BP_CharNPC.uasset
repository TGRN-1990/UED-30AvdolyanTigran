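; BP_CharNPC is an NPC character with stats, a health bar widget and a healing-item bounty on death.
; It binds to BPCharStats status updates, refreshing the life bar while alive and calling DeadNPC when dead.
; Death hides the bar, plays an animation, activates particles, then loops over a random bounty count with siren sound, Delay and BP_Item_Heal spawn, calling DestroyActor after the loop.
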(event Custom|DeadNPC
  ;[1 1 1] Bounty
  (Rendering|SetVisibility (Variables|Utilities|Transformation|GetWidget_NPC_healt) false false)
  (Components|Animation|PlayAnimation (Variables|Character|GetMesh) "/Game/Blueprints/Animation/Death_1.Death_1" false)
  (Components|Activation|Activate (Variables|Default|GetParticleSystem) false)
  (bind _returnvalue (CallFunction|MaxBountyRandomazer))
  (bind _output_get (Variables|Default|SetBounty _returnvalue))
  (for _index (range 0 (Math|Conversions|ToInteger(Byte) _output_get))
    (Audio|SpawnSound2D "/Game/Retro_8Bit_Sounds/Alarms_Sirens/Wavs/retro_alarm_siren_loop_12.retro_alarm_siren_loop_12" 1.0 1.0 0.0 0)
    (Utilities|FlowControl|Delay 1.0)
    (Game|SpawnActorfromClass "/Game/Blueprints/Arena_Object/Item/BP_Item_Heal.BP_Item_Heal_C" (Transformation|GetWorldTransform (Variables|Utilities|Transformation|GetItemSpawner)) "AdjustIfPossibleButAlwaysSpawn" 0 0))
  (Actor|DestroyActor))

(event EventBeginPlay
  (bind _bp_char_stats (Variables|Default|GetBP_Char_Stats))
  (|CallParentFunction)
  (Variables|Default|SetBP_char_Stats_reference (Variables|Default|GetBP_Char_Stats))
  (EventDispatchers|BindEventtoOnStatusUpdate (Variables|Default|GetBP_Char_Stats) (EventDispatchers|CreateEvent :!event BPonStatsUpdated))
  (CallFunction|NPCStatUpdated self false false (Variables|/Game/Blueprints/Companent/BP_Char_Stats.BP_Char_Stats_C|GetCurrentHP _bp_char_stats) (Variables|/Game/Blueprints/Companent/BP_Char_Stats.BP_Char_Stats_C|GetCurrentEP _bp_char_stats)))

(event Collision|EventActorBeginOverlap
  (params (OtherActor :type Actor%20Object%20Reference))
  (|CallParentFunction OtherActor) ; This node is disabled and will not be called.\nDrag off pins to build functionality.
)

(event EventTick
  (params (DeltaSeconds :type Float%20%28single-precision%29))
  (|CallParentFunction DeltaSeconds))

(fn ConstructionScript
  (|CallParentFunction))

(fn BPNPCStatUpdated
  (params (IsDead :type Boolean) (ItsDamage :type Boolean) (CurrentHP :type Integer) (CurrentEP :type Integer))
  (if IsDead
    (CallFunction|DeadNPC)
    (else
      (Default|ConfigLifebar (Variables|Default|GetBP_Char_Stats))
      (bind _asbp_widjet_npc_bar (Utilities|Casting|CastToBP_widjet_NPC_bar (UserInterface|GetUserWidgetObject (Variables|Utilities|Transformation|GetWidget_NPC_healt))))
      (Variables|/Game/Blueprints/BP_HUD/BP_Widjet/BP_widjet_NPC_bar.BP_widjet_NPC_bar_C|SetNPC _asbp_widjet_npc_bar self))))

(fn MaxBountyByte
  (return (Math|Conversions|ToByte(Integer) (Math|Random|RandomInteger (Math|Conversions|ToInteger(Byte) (Variables|Default|GetMax%20Bounty))))))

(fn MaxBountyRandomazer
  (return (+ (Math|Conversions|ToByte(Integer) (Math|Random|RandomInteger (Math|Conversions|ToInteger(Byte) (Variables|Default|GetMax%20Bounty)))) 1)))

(fn InvisibaleteforDead
  (Rendering|SetVisibility (Variables|Character|GetMesh) false false)
  (Rendering|SetVisibility (Variables|Utilities|Transformation|GetWidget_NPC_healt) false false))
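; Character stats component that tracks HP, EP and death state for its owner.
; It loads limits from a data table row by name; a config function also applies walk speeds.
; Damage, heal and shield events broadcast status updates, while Tick computes bar ratios.
; Reload converts HP into EP, shot costs draw on HP, and partial shield recovery writes to CurrentHP rather than CurrentEP.
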(event EventBeginPlay
  ;[1 1 1] BeginPlay
  (bind _returnvalue (Utilities|GetDataTableRow "/Game/Blueprints/Data/BP_DT_All_stats1.BP_DT_All_stats1" (Variables|Default|GetCurrenName))
    (:then
      (Variables|Default|SetMainStats _returnvalue)
      (Utilities|FlowControl|Sequence
        (:then_0
          (bind _output_get (Variables|Default|SetMaxHPCount (.MaxHP (Utilities|Struct|BreakBP_Main_Struct (Variables|Default|GetMainStats)))))
          (Variables|Default|SetCurrentHP _output_get))
        (:then_1
          (bind _output_get_2 (Variables|Default|SetMaxEPCount (.MaxEP (Utilities|Struct|BreakBP_Main_Struct (Variables|Default|GetMainStats)))))
          (Variables|Default|SetCurrentEP _output_get_2))))))

(event EventTick
  (params (DeltaSeconds :type Float%20%28single-precision%29))
  ;[1 1 1] Tick
  (Utilities|FlowControl|Sequence
    (:then_0
      (Variables|Default|SetLifebarFloat (/ (Math|Conversions|ToFloat(Integer) (Variables|Default|GetCurrentHP)) (Math|Conversions|ToFloat(Integer) (Variables|Default|GetMaxHPCount)))))
    (:then_1
      (Variables|Default|SetEnergyFloat (/ (Math|Conversions|ToFloat(Integer) (Variables|Default|GetCurrentEP)) (Math|Conversions|ToFloat(Integer) (Variables|Default|GetMaxEPCount)))))))

(event EventDamage
  (params (InDamage :type Integer) (InType :type Byte :default 0) (InCauser :type Actor%20Object%20Reference))
  ;[1 1 1] ReciveDamage
  (if (not (Variables|Default|GetIsDead))
    (bind _output_get (Variables|Default|SetCurrentHP (- (Variables|Default|GetCurrentHP) InDamage)))
    (if (> _output_get 0)
      (Variables|Default|SetIsDead false)
      (else
        (Variables|Default|SetCurrentHP 0)
        (Variables|Default|SetIsDead true)))
    (Default|CallOnStatusUpdate (Variables|Default|GetIsDead) true (Variables|Default|GetCurrentHP) (Variables|Default|GetCurrentEP))))

(event EventHealUP
  (params (MaxRecover :type Boolean) (AddHP :type Integer))
  ;[1 1 1] BP Heal UP
  (if MaxRecover
    (Variables|Default|SetCurrentHP (Variables|Default|GetMaxHPCount))
    (else
      (Variables|Default|SetCurrentHP (Math|Integer|Min(Integer) (+ AddHP (Variables|Default|GetCurrentHP)) (Variables|Default|GetMaxHPCount)))))
  (Default|CallOnStatusUpdate (Variables|Default|GetIsDead) false (Variables|Default|GetCurrentHP) (Variables|Default|GetCurrentEP)))

(event EventShieldUp
  (params (MaxRecover :type Boolean) (Add_EP :type Integer))
  ;[1 1 1] BP_ShieldUP
  (if MaxRecover
    (Variables|Default|SetCurrentEP (Variables|Default|GetMaxEPCount))
    (else
      (Variables|Default|SetCurrentHP (Math|Integer|Min(Integer) (+ Add_EP (Variables|Default|GetCurrentEP)) (Variables|Default|GetMaxEPCount)))))
  (Default|CallOnStatusUpdate (Variables|Default|GetIsDead) false (Variables|Default|GetCurrentHP) (Variables|Default|GetCurrentEP)))

(event EventReloadWeapon
  (params (Pay :type Integer))
  ;[1 1 1] ReloadWeapon
  (Variables|Default|SetCurrentHP (- (Variables|Default|GetCurrentHP) Pay))
  (if (> (+ (Variables|Default|GetCurrentEP) Pay) (Variables|Default|GetMaxEPCount))
    (Variables|Default|SetCurrentEP (Variables|Default|GetMaxEPCount))
    (else
      (Variables|Default|SetCurrentEP (+ (Variables|Default|GetCurrentEP) Pay)))))

(fn BPConfigState
  (bind _returnvalue (Utilities|GetDataTableRow "/Game/Blueprints/Data/BP_DT_All_stats1.BP_DT_All_stats1" (Variables|Default|GetCurrenName))
    (:then
      (Variables|Default|SetMainStats _returnvalue)
      (Utilities|FlowControl|Sequence
        (:then_0
          (Configuration|ConfigMove))
        (:then_1
          (CallFunction|HealUP true))
        (:then_2
          (CallFunction|ShieldUp true))
        (:then_3
          (Configuration|ConfigLifebar))))))

(fn BPConfigMove
  (bind _mainstats (Variables|Default|GetMainStats))
  (bind _maxwolkspeed (Utilities|Struct|BreakBP_Main_Struct _mainstats))
  (if (Utilities|Enum|NotEqual(Enum) (Utilities|Struct|BreakBP_Main_Struct (Variables|Default|GetMainStats)) "NewEnumerator7")
    (bind _ascharacter (Utilities|Casting|CastToCharacter (Components|GetOwner)))
    (Variables|/Script/Engine.CharacterMovementComponent|SetMaxWalkSpeed (Variables|/Script/Engine.Character|GetCharacterMovement _ascharacter) _maxwolkspeed)
    (Variables|/Script/Engine.CharacterMovementComponent|SetMaxWalkSpeedCrouched (Variables|/Script/Engine.Character|GetCharacterMovement _ascharacter) (/ _maxwolkspeed 2.0))))

(fn BPConfigLifebar
  (bind _mainstats (Variables|Default|GetMainStats))
  (bind (_maxhp _maxep) (Utilities|Struct|BreakBP_Main_Struct _mainstats))
  (return (Utilities|String|Append (Utilities|GetDisplayName (Components|GetOwner)) " / " (Utilities|String|Append (Utilities|String|ToString(Integer) (Variables|Default|GetCurrentHP)) "/" (Utilities|String|ToString(Integer) _maxhp) "HP " (Utilities|String|ToString(Integer) (Variables|Default|GetCurrentEP)) "/" (Utilities|String|ToString(Integer) _maxep) "EP "))))

(fn CheckEP
  (return (== (Variables|Default|GetCurrentHP) (Utilities|Struct|BreakBP_Main_Struct (Variables|Default|GetMainStats)))))

(fn CheckHP
  (return (== (Variables|Default|GetCurrentHP) (Utilities|Struct|BreakBP_Main_Struct (Variables|Default|GetMainStats)))))

(fn ShootingEnergyDrain
  (params (EnergyCost :type Integer))
  (if (>= (Variables|Default|GetCurrentHP) EnergyCost)
    (Variables|Default|SetCurrentHP (- (Variables|Default|GetCurrentHP) EnergyCost))
    (LocalVariables|SetShotEPC true)
    (else
      (LocalVariables|SetShotEPC false)))
  (Development|PrintString (Utilities|String|ToString(Integer) (Variables|Default|GetCurrentHP)))
  (return (LocalVariables|GetShotEPC)))
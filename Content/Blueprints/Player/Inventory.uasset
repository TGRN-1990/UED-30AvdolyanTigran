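; Player inventory Blueprint that loots the nearby items stored in an array, handling key and heal pickups.
; LootingEvent walks the array in reverse, casting each item: keys raise the parent's key count, heals add fixed HP capped at maximum, and used items are destroyed.
; Heals found at full HP move to a mirror array, appended back after the loop so they remain lootable.
; A pickup sound plays even for skipped heals.
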(event EventBeginPlay)

(event EventTick
  (params (DeltaSeconds :type Float%20%28single-precision%29)))

(fn HealOverHealing
  (bind _selfparent (Variables|Default|GetSelfParent))
  (bind _bp_char_stats (Variables|/Game/Blueprints/Base/BP_Character_Base.BP_Character_Base_C|GetBP_Char_Stats _selfparent))
  (bind _maxhpcount (Variables|/Game/Blueprints/Companent/BP_Char_Stats.BP_Char_Stats_C|GetMaxHPCount _bp_char_stats))
  (bind _output_get (Variables|Default|SetOverHeal (<= (Variables|/Game/Blueprints/Companent/BP_Char_Stats.BP_Char_Stats_C|GetMaxHPCount _bp_char_stats) (Variables|/Game/Blueprints/Companent/BP_Char_Stats.BP_Char_Stats_C|GetCurrentHP _bp_char_stats))))
  (if _output_get
    ;[1 1 1] SaveOverHeal Elements
    (Utilities|Array|AddUnique (Variables|Default|GetNearItemsMirror) (Utilities|Array|Get(acopy) (Variables|Default|GetNearItemsArrow) (Variables|Default|GetItemIndex)))
    (Utilities|Array|RemoveIndex (Variables|Default|GetNearItemsArrow) (Variables|Default|GetItemIndex))
    (return (Variables|Default|GetOverHeal))
    (else
      (Variables|/Game/Blueprints/Companent/BP_Char_Stats.BP_Char_Stats_C|SetCurrentHP _bp_char_stats (+ 50 (Variables|/Game/Blueprints/Companent/BP_Char_Stats.BP_Char_Stats_C|GetCurrentHP _bp_char_stats)))
      (if (> (Variables|/Game/Blueprints/Companent/BP_Char_Stats.BP_Char_Stats_C|GetCurrentHP _bp_char_stats) _maxhpcount)
        (Variables|/Game/Blueprints/Companent/BP_Char_Stats.BP_Char_Stats_C|SetCurrentHP _bp_char_stats _maxhpcount)
        (return (Variables|Default|GetOverHeal))))))

(fn LootingEvent
  (bind _selfparent (Variables|Default|GetSelfParent))
  (Utilities|Array|Clear (Variables|Default|GetNearItemsMirror))
  (bind (_arrayindex _arrayelement) (Utilities|Array|ReverseforEachLoop (Variables|Default|GetNearItemsArrow) :!label _label)
    (:LoopBody
      (Variables|Default|SetItemIndex _arrayindex)
      (Utilities|FlowControl|Sequence
        (:then_0
          (bind _asbp_item_key (Utilities|Casting|CastToBP_item_key _arrayelement))
          (Variables|/Game/Blueprints/Base/BP_Character_Base.BP_Character_Base_C|SetItemKeyCount _selfparent (+ (Variables|/Game/Blueprints/Base/BP_Character_Base.BP_Character_Base_C|GetItemKeyCount _selfparent) 1))
          (Actor|DestroyActor _asbp_item_key))
        (:then_1
          (bind _asbp_item_heal (Utilities|Casting|CastToBP_Item_Heal _arrayelement))
          (bind _overheal (CallFunction|HealOverHealing))
          (if _overheal
            _
            (else
              (Actor|DestroyActor _asbp_item_heal)))))
      (Audio|SpawnSound2D "/Game/Retro_8Bit_Sounds/Jumping/Cues/retro_jump_bounce_13_Cue.retro_jump_bounce_13_Cue" 1.0 1.0 0.0 0)
      (goto _label))
    (:Completed
      (Utilities|Array|AppendArray (Variables|Default|GetNearItemsArrow) (Variables|Default|GetNearItemsMirror)))))
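; Player character Blueprint that ties together stats, stealth noise, an arrow weapon, lives and save/load.
; BeginPlay starts a one-second noise loop for AI perception, spawns an arrow that Tick pins to ArrowWeapon, and runs GameInstance level loaders.
; Tick lowers noise loudness while crouched and triggers EndHero at zero HP, spending a life (Arsenal) to reload a checkpoint or notifying the controller.
; Capsule overlaps track nearby items for Inventory.
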(event OnComponentBeginOverlap(CapsuleComponent)
  (params (OverlappedComponent :type Primitive%20Component%20Object%20Reference) (OtherActor :type Actor%20Object%20Reference) (OtherComp :type Primitive%20Component%20Object%20Reference) (OtherBodyIndex :type Integer) (bFromSweep :type Boolean) (SweepResult :type Hit%20Result%20Structure%20%28by%20ref%29))
  ;[1 1 1] ItemSensor
  (bind _asbp_0_item_base (Utilities|Casting|CastToBP_0_Item_Base OtherActor))
  (Utilities|Array|AddUnique (Variables|/Game/Blueprints/Player/Inventory.Inventory_C|GetNearItemsArrow (Variables|Default|GetInventory)) _asbp_0_item_base))

(event OnComponentEndOverlap(CapsuleComponent)
  (params (OverlappedComponent :type Primitive%20Component%20Object%20Reference) (OtherActor :type Actor%20Object%20Reference) (OtherComp :type Primitive%20Component%20Object%20Reference) (OtherBodyIndex :type Integer))
  ;[1 1 1] ItemSensor
  (bind _asbp_0_item_base (Utilities|Casting|CastToBP_0_Item_Base OtherActor))
  (Utilities|Array|RemoveItem (Variables|/Game/Blueprints/Player/Inventory.Inventory_C|GetNearItemsArrow (Variables|Default|GetInventory)) _asbp_0_item_base))

(event Custom|EndHero
  ;[1 1 1] DeadHero
  (if (!= (Variables|Default|GetArsenal) 0)
    (Variables|Default|SetArsenal (- (Variables|Default|GetArsenal) 1))
    (CallFunction|UpdateStatus)
    (bind _asbp_save_game_inst (Utilities|Casting|CastToBP_SaveGameInst (Game|GetGameInstance)))
    (Default|CheckPointsLoad _asbp_save_game_inst)
    (else
      (Default|DeadHero (Variables|Default|GetTargetControllChar)))))

(event EventBeginPlay
  (bind _bp_char_stats (Variables|Default|GetBP_Char_Stats))
  ;[1 1 1] Event BeginPlay
  (|CallParentFunction)
  (bind _asbp_char_controlls (Utilities|Casting|CastToBP_CharControlls (Game|GetPlayerController 0)))
  (Variables|Default|SetTargetControllChar _asbp_char_controlls)
  (Utilities|FlowControl|Sequence
    (:then_0
      (Utilities|FlowControl|Delay 1.0 :!label _label)
      (Class|AISenseHearing|ReportNoiseEvent (Transformation|GetWorldLocation (Variables|Default|GetCapsuleComponent)) (Variables|Default|GetLoudness_1or3/4) self 0.0 "None")
      (goto _label))
    (:then_1
      (EventDispatchers|BindEventtoOnStatusUpdate (Variables|Default|GetBP_Char_Stats) (EventDispatchers|CreateEvent :!event BPPlayerStatUpdated))
      (CallFunction|UpdateStatus)
      (Components|Activation|Activate (Variables|Default|GetAIPerceptionStimuliSource) true))
    (:then_2
      (bind _returnvalue (Game|SpawnActorfromClass "/Game/Blueprints/Magik(Weapon)/Spells/Arrow.Arrow_C" (Transformation|GetWorldTransform (Variables|Default|GetArrow_weapon)) "Undefined" 0 0))
      (bind _output_get (Variables|Default|SetMagika _returnvalue))
      (Variables|/Game/Blueprints/Base/BP_CharControlls.BP_CharControlls_C|SetSelect_Magik (Variables|Default|GetTargetControllChar) _output_get)
      (Variables|Default|SetWeapon%20Activate true))
    (:then_3
      (bind _asbp_save_game_inst (Utilities|Casting|CastToBP_SaveGameInst (Game|GetGameInstance)))
      (Default|LevelPostLoader _asbp_save_game_inst)
      (Default|LevelNextLoader _asbp_save_game_inst)
      (CallFunction|PlayerStatUpdated false false (Variables|/Game/Blueprints/Companent/BP_Char_Stats.BP_Char_Stats_C|GetCurrentHP _bp_char_stats) (Variables|/Game/Blueprints/Companent/BP_Char_Stats.BP_Char_Stats_C|GetCurrentEP _bp_char_stats)))))

(event EventTick
  (params (DeltaSeconds :type Float%20%28single-precision%29))
  ;[1 1 1] EventTickSensor
  (Utilities|FlowControl|Sequence
    (:then_0
      (CallFunction|CrouchSillence))
    (:then_1
      (Default|CrouchandJump self))
    (:then_2
      (Variables|Default|SetCharCoord (Transformation|GetActorLocation)))
    (:then_3
      (Variables|Default|SetCharToord (Transformation|GetActorTransform)))
    (:then_4
      (if (not (> (Variables|/Game/Blueprints/Companent/BP_Char_Stats.BP_Char_Stats_C|GetCurrentHP (Variables|Default|GetBP_Char_Stats)) 0))
        (CallFunction|EndHero)))
    (:then_5
      (if (Variables|Default|GetWeapon%20Activate)
        (Transformation|SetActorTransform (Variables|Default|GetMagika) (Transformation|GetWorldTransform (Variables|Default|GetArrow_weapon)) true true)))))

(fn ConstructionScript
  (|CallParentFunction))

(fn BPPlayerStatUpdated
  (params (IsDead :type Boolean) (ItsDamage :type Boolean) (CurrentHP :type Integer) (CurrentEP :type Integer))
  (if IsDead
    (CallFunction|EndHero)
    (else
      (bind _asbp_widjet_bar (Utilities|Casting|CastToBP_widjet_bar (UserInterface|GetUserWidgetObject (Variables|Default|GetWidgetChar))))
      (Variables|/Game/Blueprints/BP_HUD/BP_Widjet/BP_widjet_bar.BP_widjet_bar_C|SetCharPlayerWijet _asbp_widjet_bar self)
      (Variables|Default|SetLife (Utilities|String|Append (Utilities|String|ToString(Byte) (Variables|Default|GetArsenal)) " Life" " / " (Utilities|String|ToString(Byte) (Variables|Default|GetItemKeyCount)) " Key ")))))

(fn CrouchSillence
  (bind _returnvalue (Game|GetInstigatorController))
  (if (Utilities|DoesObjectImplementInterface _returnvalue "/Game/Blueprints/Base/BPI_Controls.BPI_Controls_C")
    (bind _outcrouch (Class|BPIControls|WalkJumpCrouch(Message) _returnvalue))
    (if _outcrouch
      (Variables|Default|SetLoudness_1or3/4 0.75)
      (else
        (Variables|Default|SetLoudness_1or3/4 1.0)))))

(fn CheckforSave
  (params (CharPlayer :type BP%20Char%20Player%20Object%20Reference))
  (Variables|Default|SetCharPlayer CharPlayer)
  (bind _returnvalue (Game|GetCurrentLevelName true))
  (return _returnvalue (Transformation|GetActorLocation (Variables|Default|GetCharPlayer)) (Transformation|GetActorTransform (Variables|Default|GetCharPlayer)) (Variables|/Game/Blueprints/Companent/BP_Char_Stats.BP_Char_Stats_C|GetCurrentHP (Variables|/Game/Blueprints/Base/BP_Character_Base.BP_Character_Base_C|GetBP_Char_Stats (Variables|Default|GetCharPlayer))) (Variables|/Game/Blueprints/Companent/BP_Char_Stats.BP_Char_Stats_C|GetCurrentEP (Variables|/Game/Blueprints/Base/BP_Character_Base.BP_Character_Base_C|GetBP_Char_Stats (Variables|Default|GetCharPlayer))) (Variables|BP_CharPlayer_C|GetArsenal (Variables|Default|GetCharPlayer))))

(fn CheckforLoadChar
  (params (CurrentHP :type Integer) (CurrentEP :type Integer) (Arsenal :type Byte) (Target :type BP%20Char%20Player%20Object%20Reference))
  (bind _bp_char_stats (Variables|Default|GetBP_Char_Stats))
  (Variables|/Game/Blueprints/Companent/BP_Char_Stats.BP_Char_Stats_C|SetCurrentHP _bp_char_stats CurrentHP)
  (Variables|/Game/Blueprints/Companent/BP_Char_Stats.BP_Char_Stats_C|SetCurrentEP _bp_char_stats CurrentEP)
  (Variables|Default|SetArsenal Arsenal))

(fn CheckforLoadCoor
  (params (PlayerVector :type Vector) (PlayerTransforn :type Transform) (Target :type BP%20Char%20Player%20Object%20Reference))
  (Transformation|AddActorWorldOffset Target PlayerVector false true)
  (Transformation|SetActorRelativeTransform Target PlayerTransforn false true))

(fn UpdateStatus
  (bind _bp_char_stats (Variables|Default|GetBP_Char_Stats))
  (CallFunction|PlayerStatUpdated self false false (Variables|/Game/Blueprints/Companent/BP_Char_Stats.BP_Char_Stats_C|GetCurrentHP _bp_char_stats) (Variables|/Game/Blueprints/Companent/BP_Char_Stats.BP_Char_Stats_C|GetCurrentEP _bp_char_stats)))
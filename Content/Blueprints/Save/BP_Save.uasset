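; BP_Save is a save data object that holds the current level, a vector, a transform, HP, EP and the arsenal.
; SaveInput writes those values into its own variables, converting the level to a Name.
; LoadOutput returns the same fields read from a passed-in TargetSlot rather than from itself.
; Neither function performs slot or disk operations; both only move data in and out of variables.
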(fn SaveInput
  (params (Level :type String) (Vector :type Vector) (Transform :type Transform) (HP :type Integer) (EP :type Integer) (Arsenal :type Byte))
  (Variables|Default|SetSv-Level (Utilities|String|StringToName Level))
  (Variables|Default|SetSv-Lock Vector)
  (Variables|Default|SetSv-T-Lock Transform)
  (Variables|Default|SetSv-HP HP)
  (Variables|Default|SetSv-EP EP)
  (Variables|Default|SetSv-Arsenal Arsenal))

(fn LoadOutput
  (params (TargetSlot :type BP%20Save%20Object%20Reference))
  (return (Variables|BP_Save_C|GetSv-Level TargetSlot) (Variables|BP_Save_C|GetSv-HP TargetSlot) (Variables|BP_Save_C|GetSv-EP TargetSlot) (Variables|BP_Save_C|GetSv-Arsenal TargetSlot) (Variables|BP_Save_C|GetSv-Lock TargetSlot) (Variables|BP_Save_C|GetSv-T-Lock TargetSlot)))
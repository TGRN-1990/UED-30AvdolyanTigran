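; Save-system game instance that handles manual save slots, checkpoints and level transitions for BP_CharPlayer through BP_Save objects.
; Saves capture level, HP, EP, arsenal and position, while checkpoint reloads refill HP and restore only position.
; Level loads copy slot data into a temporary slot and set a flag before OpenLevel.
; Post-load events then restore character stats, plus position for slot loads but not next-level transitions.
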(event Custom|CheckPointsLoad
  ;[1 1 1] Система Сохранения
  (bind _asbp_char_player (Utilities|Casting|CastToBP_CharPlayer (Game|Player|GetPlayerPawn 0)))
  (Variables|/Game/Blueprints/Companent/BP_Char_Stats.BP_Char_Stats_C|SetCurrentHP (Variables|/Game/Blueprints/Base/BP_Character_Base.BP_Character_Base_C|GetBP_Char_Stats _asbp_char_player) (Variables|/Game/Blueprints/Companent/BP_Char_Stats.BP_Char_Stats_C|GetMaxHPCount (Variables|/Game/Blueprints/Base/BP_Character_Base.BP_Character_Base_C|GetBP_Char_Stats _asbp_char_player)))
  (CallFunction|LoadSlotFunCoordinate (Variables|Default|GetCheckPointSlot) (Variables|Default|GetChekPoint)))

(event Custom|LevelNextLoader
  ;[1 1 1] Система Сохранения
  (if (Variables|Default|GetSlotLevelLoader)
    (CallFunction|LoadSlotFunChar (Variables|Default|GetTempleSlot) (Variables|Default|GetTempleSlotName))
    (Variables|Default|SetSlotLevelLoader false)))

(event Custom|CheckPointsSave
  (params (CPVector :type Vector) (CPTransporation :type Transform))
  (bind _chekpoint (Variables|Default|GetChekPoint))
  ;[1 1 1] Система Сохранения
  (bind _returnvalue (CallFunction|CreateSlot _chekpoint))
  (bind _output_get (Variables|Default|SetCheckPointSlot _returnvalue))
  (CallFunction|SaveCheckpoint CPVector CPTransporation _output_get _chekpoint))

(event Custom|LoadSlot
  (params (T-SaveSlot :type BP%20Save%20Object%20Reference) (T-SaveSlotName :type String))
  ;[1 1 1] Система Сохранения
  (CallFunction|LoadSlotFunLevel T-SaveSlot T-SaveSlotName))

(event Custom|SaveSlot
  (params (T-SaveSlot :type BP%20Save%20Object%20Reference) (T-StringSlot :type String))
  ;[1 1 1] Система Сохранения
  (CallFunction|SaveSlotFun T-SaveSlot T-StringSlot))

(event Custom|LevelPostLoader
  (bind _templeslot (Variables|Default|GetTempleSlot))
  (bind _templeslotname (Variables|Default|GetTempleSlotName))
  ;[1 1 1] Система Сохранения
  (if (Variables|Default|GetSlotPostLoader)
    (CallFunction|LoadSlotFunCoordinate _templeslot _templeslotname)
    (CallFunction|LoadSlotFunChar _templeslot _templeslotname)
    (Variables|Default|SetSlotPostLoader false)))

(event Custom|LoadNextLevel
  (params (T-SaveSlot :type BP%20Save%20Object%20Reference) (T-SaveSlotName :type String) (LevelTarget :type Name))
  ;[1 1 1] Система Сохранения
  (CallFunction|LoadSlotFunNextLevel T-SaveSlot T-SaveSlotName LevelTarget))

(fn ConstructionScript)

(fn CreateSlot
  (params (SlotName :type String))
  (bind _output_get (LocalVariables|SetInitName SlotName))
  (bind _returnvalue (SaveGame|DoesSaveGameExist _output_get))
  (if _returnvalue
    _
    (else
      (bind _returnvalue_2 (SaveGame|CreateSaveGameObject "/Game/Blueprints/Save/BP_Save.BP_Save_C"))
      (SaveGame|SaveGametoSlot _returnvalue_2 (LocalVariables|GetInitName))))
  (bind _returnvalue_3 (SaveGame|LoadGamefromSlot (LocalVariables|GetInitName)))
  (bind _asbp_save (Utilities|Casting|CastToBP_Save _returnvalue_3))
  (bind _output_get_2 (LocalVariables|SetInitSlot _asbp_save))
  (return _output_get_2))

(fn SaveSlotFun
  (params (SaveSlot :type BP%20Save%20Object%20Reference) (SlotName :type String))
  (bind _asbp_char_player (Utilities|Casting|CastToBP_CharPlayer (Game|GetPlayerCharacter 0)))
  (bind (_levelname _playervector _playertransform _current_hp _current_ep _arsenal) (Default|CheckforSave _asbp_char_player _asbp_char_player))
  (Default|SaveInput SaveSlot _levelname _current_hp _current_ep _arsenal _playervector _playertransform)
  (SaveGame|SaveGametoSlot SaveSlot SlotName)
  (return))

(fn LoadSlotFunChar
  (params (Target%20Slot :type BP%20Save%20Object%20Reference) (TargetSlotName :type String))
  (bind _returnvalue (SaveGame|LoadGamefromSlot TargetSlotName))
  (bind _asbp_save (Utilities|Casting|CastToBP_Save _returnvalue))
  (bind (_level _hp _ep _arsenal) (Default|LoadOutput _asbp_save _asbp_save))
  (bind _asbp_char_player (Utilities|Casting|CastToBP_CharPlayer (Game|GetPlayerCharacter 0)))
  (Default|CheckforLoadChar _asbp_char_player _hp _ep _arsenal _asbp_char_player))

(fn LoadSlotFunLevel
  (params (Target%20Slot :type BP%20Save%20Object%20Reference) (TargetSlotName :type String))
  (LocalVariables|SetLoadSlotFun Target%20Slot)
  (LocalVariables|SetLoadSlotName TargetSlotName)
  (bind _returnvalue (CallFunction|CreateSlot (Variables|Default|GetTempleSlotName)))
  (Variables|Default|SetTempleSlot _returnvalue)
  (bind _returnvalue_2 (SaveGame|LoadGamefromSlot TargetSlotName))
  (bind _asbp_save (Utilities|Casting|CastToBP_Save _returnvalue_2))
  (bind (_level _hp _ep _arsenal _lock _transform) (Default|LoadOutput _asbp_save _asbp_save))
  (LocalVariables|SetLevel _level)
  (Default|SaveInput (Variables|Default|GetTempleSlot) "" _hp _ep _arsenal _lock _transform)
  (SaveGame|SaveGametoSlot (Variables|Default|GetTempleSlot) (Variables|Default|GetTempleSlotName))
  (Variables|Default|SetSlotPostLoader true)
  (Game|OpenLevel(byName) (LocalVariables|GetLevel)))

(fn LoadSlotFunCoordinate
  (params (Target%20Slot :type BP%20Save%20Object%20Reference) (TargetSlotName :type String))
  (bind _returnvalue (SaveGame|LoadGamefromSlot TargetSlotName))
  (bind _asbp_save (Utilities|Casting|CastToBP_Save _returnvalue))
  (bind (_level _hp _ep _arsenal _lock _transform) (Default|LoadOutput _asbp_save _asbp_save))
  (bind _asbp_char_player (Utilities|Casting|CastToBP_CharPlayer (Game|GetPlayerCharacter 0)))
  (Default|CheckforLoadCoor _asbp_char_player _lock _transform _asbp_char_player))

(fn MenuVisible
  (bind _asbp_char_controlls (Utilities|Casting|CastToBP_CharControlls (Game|GetPlayerController 0)))
  (Default|WInit _asbp_char_controlls)
  (bind _asbp_char_player (Utilities|Casting|CastToBP_CharPlayer (Game|Player|GetPlayerPawn 0)))
  (Rendering|SetVisibility (Variables|/Game/Blueprints/Player/BP_CharPlayer.BP_CharPlayer_C|GetWidgetChar _asbp_char_player) true false))

(fn Slot?
  (params (SlotName :type String))
  (bind _output_get (LocalVariables|SetInitName SlotName))
  (bind _returnvalue (SaveGame|DoesSaveGameExist _output_get))
  (return _returnvalue))

(fn LoadSlotFunNextLevel
  (params (Target%20Slot :type BP%20Save%20Object%20Reference) (TargetSlotName :type String) (TargetLevel :type Name))
  (LocalVariables|SetLevel TargetLevel)
  (LocalVariables|SetLoadSlotFun Target%20Slot)
  (LocalVariables|SetLoadSlotName TargetSlotName)
  (bind _returnvalue (CallFunction|CreateSlot (Variables|Default|GetTempleSlotName)))
  (Variables|Default|SetTempleSlot _returnvalue)
  (bind _returnvalue_2 (SaveGame|LoadGamefromSlot TargetSlotName))
  (bind _asbp_save (Utilities|Casting|CastToBP_Save _returnvalue_2))
  (bind (_level _hp _ep _arsenal _lock _transform) (Default|LoadOutput _asbp_save _asbp_save))
  (Default|SaveInput (Variables|Default|GetTempleSlot) "" _hp _ep _arsenal _lock _transform)
  (SaveGame|SaveGametoSlot (Variables|Default|GetTempleSlot) (Variables|Default|GetTempleSlotName))
  (Variables|Default|SetSlotLevelLoader true)
  (Game|OpenLevel(byName) (LocalVariables|GetLevel)))

(fn SaveCheckpoint
  (params (CoorV :type Vector) (CoorT :type Transform) (SaveSlot :type BP%20Save%20Object%20Reference) (SlotName :type String))
  (bind _asbp_char_player (Utilities|Casting|CastToBP_CharPlayer (Game|GetPlayerCharacter 0)))
  (bind (_levelname _playervector _playertransform _current_hp _current_ep _arsenal) (Default|CheckforSave _asbp_char_player _asbp_char_player))
  (Default|SaveInput SaveSlot _levelname _current_hp _current_ep _arsenal CoorV CoorT)
  (SaveGame|SaveGametoSlot SaveSlot SlotName)
  (return))
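; BP_Bullet_Base_enemy is, by its name and location, the base Blueprint for enemy bullets in the Magik weapon set.
; On BeginPlay it looks up its BullettType row in the BP_Magik_all_stats data table and caches the row plus cost, damage, cast time, cooldown and auto-reload.
; DamageDealer only returns zero, and the graphs contain no movement or hit logic.
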(event EventBeginPlay
  (bind _returnvalue (Utilities|GetDataTableRow "/Game/Blueprints/Data/BP_Magik_all_stats.BP_Magik_all_stats" (Variables|Default|GetBullettType))
    (:then
      (bind _output_get (Variables|Default|SetBulletData _returnvalue))
      (Variables|Default|SetCost (.Cost (Utilities|Struct|BreakMagik_Struct _output_get)))
      (Variables|Default|SetDamage (.Damage (Utilities|Struct|BreakMagik_Struct _output_get)))
      (Variables|Default|SetCast%20Time (.CastTime (Utilities|Struct|BreakMagik_Struct _output_get)))
      (Variables|Default|SetCooldown (.Cooldown (Utilities|Struct|BreakMagik_Struct _output_get)))
      (Variables|Default|SetAuto%20Reload (.AutoReload (Utilities|Struct|BreakMagik_Struct _output_get))))))

(event EventTick
  (params (DeltaSeconds :type Float%20%28single-precision%29)))

(fn ConstructionScript)

(fn DamageDealer
  (return 0))
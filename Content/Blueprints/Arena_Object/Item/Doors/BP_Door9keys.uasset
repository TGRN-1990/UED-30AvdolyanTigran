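; A door actor that opens only when the player holds at least KeyNeed keys, otherwise printing a Russian "keys needed" message.
; An overlap box arms it for actors implementing BPI_looter and stores the player reference used by UseObject.
; A timeline rotates the mesh yaw, with a dot product against the player's position picking the swing direction.
; Using it again reverses the timeline to close it; keys are not consumed.
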(event OnComponentBeginOverlap(CollBox)
  (params (OverlappedComponent :type Primitive%20Component%20Object%20Reference) (OtherActor :type Actor%20Object%20Reference) (OtherComp :type Primitive%20Component%20Object%20Reference) (OtherBodyIndex :type Integer) (bFromSweep :type Boolean) (SweepResult :type Hit%20Result%20Structure%20%28by%20ref%29))
  (if (Utilities|DoesObjectImplementInterface OtherActor "/Game/Blueprints/Base/BPI_looter.BPI_looter_C")
    (Variables|Default|SetDoor_activated true)
    (bind _selfref (Class|BPILooter|SelfRef(Message) OtherActor))
    (Variables|Default|SetPlayerRef _selfref)))

(event OnComponentEndOverlap(CollBox)
  (params (OverlappedComponent :type Primitive%20Component%20Object%20Reference) (OtherActor :type Actor%20Object%20Reference) (OtherComp :type Primitive%20Component%20Object%20Reference) (OtherBodyIndex :type Integer))
  (if (Utilities|DoesObjectImplementInterface OtherActor "/Game/Blueprints/Base/BPI_looter.BPI_looter_C")
    (Variables|Default|SetDoor_activated false)
    (Class|BPILooter|SelfRef(Message) OtherActor)))

(event EventUseObject
  (params (UserPlayer :type BP%20Character%20Base%20Object%20Reference))
  (bind _box (Variables|Default|GetBox))
  (if (Variables|Default|GetDoor_activated)
    (if (>= (Variables|/Game/Blueprints/Base/BP_Character_Base.BP_Character_Base_C|GetItemKeyCount (Variables|Default|GetPlayerRef)) (Variables|Default|GetKeyNeed))
      (if (Variables|Default|GetIsDoorClosed)
        (Variables|Default|SetIsDoorClosed false)
        (Variables|Default|SetDotProduct (Math|Vector|DotProduct (Math|Vector|Normalize (- (Transformation|GetWorldLocation _box) (Transformation|GetActorLocation (Variables|Default|GetPlayerRef)))) (Math|Vector|GetForwardVector _box)))
        (bind (_direction _newtrack_0) (Timeline|Timeline_0 Play)
          (:Update
            (Transformation|SetRelativeRotation (Variables|Default|GetStaticMesh) (Math|Rotator|MakeRotator 0.0 0.0 (Math|Float|Lerp 0.0 (Math|Float|SelectFloat -9e+01 9e+01 (>= (Variables|Default|GetDotProduct) 0.0)) _newtrack_0)) false false))
          (:Finished
            (switch Utilities|FlowControl|Switch|SwitchonETimelineDirection _direction
              (:Backward
                (Variables|Default|SetIsDoorClosed true)))))
        (else
          (Timeline|Timeline_0 Reverse)))
      (else
        (Development|PrintString (Utilities|String|Append " Нужно ключей " (Utilities|String|ToString(Byte) (Variables|Default|GetKeyNeed))))))))

(fn ConstructionScript)

(fn ItemType
  (return))
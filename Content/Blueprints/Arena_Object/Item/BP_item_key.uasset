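; Key item pickup that grants keys to the player who uses it.
; UseObject adds its KeyInWeb amount to the user's ItemKeyCount, refreshes status through UpdateStatus when the user is a BP_CharPlayer, then destroys the actor either way.
; BeginPlay, overlap and Tick are disabled stubs, so all of its own logic runs from UseObject.
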(event EventBeginPlay
  (|CallParentFunction) ; This node is disabled and will not be called.\nDrag off pins to build functionality.
)

(event Collision|EventActorBeginOverlap
  (params (OtherActor :type Actor%20Object%20Reference))
  (|CallParentFunction OtherActor) ; This node is disabled and will not be called.\nDrag off pins to build functionality.
)

(event EventTick
  (params (DeltaSeconds :type Float%20%28single-precision%29))
  (|CallParentFunction DeltaSeconds) ; This node is disabled and will not be called.\nDrag off pins to build functionality.
)

(event EventUseObject
  (params (UserPlayer :type BP%20Character%20Base%20Object%20Reference))
  (Variables|/Game/Blueprints/Base/BP_Character_Base.BP_Character_Base_C|SetItemKeyCount UserPlayer (+ (Variables|/Game/Blueprints/Base/BP_Character_Base.BP_Character_Base_C|GetItemKeyCount UserPlayer) (Variables|Default|GetKeyInWeb)))
  (bind _asbp_char_player (Utilities|Casting|CastToBP_CharPlayer UserPlayer)
    (:then
      (Default|UpdateStatus _asbp_char_player)
      (Actor|DestroyActor))
    (:CastFailed
      (Actor|DestroyActor))))

(fn ConstructionScript
  (|CallParentFunction))
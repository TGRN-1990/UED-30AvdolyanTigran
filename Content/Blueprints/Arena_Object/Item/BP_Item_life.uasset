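; BP_Item_life is an arena item that a BP_CharPlayer consumes through the UseObject event.
; On use it adds one to the player's Arsenal, calls UpdateStatus and destroys itself.
; A separate HealOverHealing function raises CurrentHP, clamps it to MaxHPCount and reports whether HP was already full, but UseObject does not call it.
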(event Collision|EventActorBeginOverlap
  (params (OtherActor :type Actor%20Object%20Reference))
  (|CallParentFunction OtherActor) ; This node is disabled and will not be called.\nDrag off pins to build functionality.
)

(event EventTick
  (params (DeltaSeconds :type Float%20%28single-precision%29))
  (|CallParentFunction DeltaSeconds) ; This node is disabled and will not be called.\nDrag off pins to build functionality.
)

(event EventUseObject
  (params (UserPlayer :type BP%20Character%20Base%20Object%20Reference))
  (bind _asbp_char_player (Utilities|Casting|CastToBP_CharPlayer UserPlayer))
  (Variables|/Game/Blueprints/Player/BP_CharPlayer.BP_CharPlayer_C|SetArsenal _asbp_char_player (+ (Variables|/Game/Blueprints/Player/BP_CharPlayer.BP_CharPlayer_C|GetArsenal _asbp_char_player) 1))
  (Default|UpdateStatus _asbp_char_player)
  (Actor|DestroyActor))

(fn ConstructionScript
  (|CallParentFunction))

(fn HealOverHealing
  (params (HealP :type Integer) (Player :type BP%20Character%20Base%20Object%20Reference))
  (bind _bp_char_stats (Variables|/Game/Blueprints/Base/BP_Character_Base.BP_Character_Base_C|GetBP_Char_Stats Player))
  (bind _maxhpcount (Variables|/Game/Blueprints/Companent/BP_Char_Stats.BP_Char_Stats_C|GetMaxHPCount _bp_char_stats))
  (LocalVariables|SetHealPower HealP)
  (bind _output_get (Variables|Default|SetOverHeal (<= (Variables|/Game/Blueprints/Companent/BP_Char_Stats.BP_Char_Stats_C|GetMaxHPCount _bp_char_stats) (Variables|/Game/Blueprints/Companent/BP_Char_Stats.BP_Char_Stats_C|GetCurrentHP _bp_char_stats))))
  (if _output_get
    _
    (else
      (Variables|/Game/Blueprints/Companent/BP_Char_Stats.BP_Char_Stats_C|SetCurrentHP _bp_char_stats (+ (LocalVariables|GetHealPower) (Variables|/Game/Blueprints/Companent/BP_Char_Stats.BP_Char_Stats_C|GetCurrentHP _bp_char_stats)))
      (if (> (Variables|/Game/Blueprints/Companent/BP_Char_Stats.BP_Char_Stats_C|GetCurrentHP _bp_char_stats) _maxhpcount)
        (Variables|/Game/Blueprints/Companent/BP_Char_Stats.BP_Char_Stats_C|SetCurrentHP _bp_char_stats _maxhpcount))))
  (return (Variables|Default|GetOverHeal)))
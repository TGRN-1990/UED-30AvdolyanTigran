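; BP_Target is a damageable target object in the arena that shows its health and destroys itself on death.
; Weapon overlaps through BPI_Weapon and engine damage carrying a BP_DamageTypeObject both feed the BPCharStats component.
; Its status-update delegate refreshes the target text and hands the actor to the NPC health-bar widget.
; On death the text shows a dead message, an alarm sound plays, and the actor is destroyed after a short delay.
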(event OnComponentBeginOverlap(targetcollbox)
  (params (OverlappedComponent :type Primitive%20Component%20Object%20Reference) (OtherActor :type Actor%20Object%20Reference) (OtherComp :type Primitive%20Component%20Object%20Reference) (OtherBodyIndex :type Integer) (bFromSweep :type Boolean) (SweepResult :type Hit%20Result%20Structure%20%28by%20ref%29))
  (if (Utilities|DoesObjectImplementInterface OtherActor "/Game/Blueprints/Magik(Weapon)/BPI_Weapon.BPI_Weapon_C")
    (bind _damage (Class|BPIWeapon|DamageDealer(Message) OtherActor))
    (Default|ReceiveDamage (Variables|Default|GetBP_Char_Stats) _damage)))

(event Custom|DeadDelay
  (Audio|SpawnSound2D "/Game/Retro_8Bit_Sounds/Alarms_Sirens/Wavs/retro_alarm_siren_loop_12.retro_alarm_siren_loop_12" 1.0 1.0 0.0 0)
  (Utilities|FlowControl|Delay 1.0)
  (Actor|DestroyActor))

(event EventBeginPlay
  (bind _bp_char_stats (Variables|Default|GetBP_Char_Stats))
  (EventDispatchers|BindEventtoOnStatusUpdate (Variables|Default|GetBP_Char_Stats) (EventDispatchers|CreateEvent :!event BPonStatsUpdated))
  (CallFunction|OnStatsUpdated self false false (Variables|/Game/Blueprints/Companent/BP_Char_Stats.BP_Char_Stats_C|GetCurrentHP _bp_char_stats) (Variables|/Game/Blueprints/Companent/BP_Char_Stats.BP_Char_Stats_C|GetCurrentEP _bp_char_stats)))

(fn ConstructionScript)

(fn ReceiveAnyDamage
  (params (Damage :type Float%20%28single-precision%29) (DamageType :type Damage%20Type%20Object%20Reference) (InstigatedBy :type Controller%20Object%20Reference) (DamageCauser :type Actor%20Object%20Reference))
  (bind _asbp_damage_type_object (Utilities|Casting|CastToBP_DamageTypeObject DamageType))
  (Default|ReceiveDamage (Variables|Default|GetBP_Char_Stats) (Variables|Default|GetDamage) (Variables|/Game/Blueprints/Object/BP_DamageTypeObject.BP_DamageTypeObject_C|GetDamageType _asbp_damage_type_object) DamageCauser))

(fn BPonStatsUpdated
  (params (IsDead :type Boolean) (ItsDamage :type Boolean) (CurrentHP :type Integer) (CurrentEP :type Integer))
  (if IsDead
    (Rendering|Components|TextRender|SetText (Variables|Default|GetTargetText) (Utilities|Text|ToText(String) (Utilities|String|Append (Utilities|GetObjectName self) "  " (Variables|Default|GetTetxDead))))
    (CallFunction|DeadDelay)
    (else
      (bind _lifebare (Default|ConfigLifebar (Variables|Default|GetBP_Char_Stats)))
      (Rendering|Components|TextRender|SetText (Variables|Default|GetTargetText) (Utilities|Text|ToText(String) _lifebare))
      (bind _asbp_widjet_npctarget_bar (Utilities|Casting|CastToBP_widjet_NPCTarget_bar (UserInterface|GetUserWidgetObject (Variables|Default|GetWidget_NPC_healt))))
      (Variables|/Game/Blueprints/BP_HUD/BP_Widjet/BP_widjet_NPCTarget_bar.BP_widjet_NPCTarget_bar_C|SetNPC_target _asbp_widjet_npctarget_bar self))))
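; Base character Blueprint that wires a stats component and inventory to a shared set of character functions.
; BeginPlay registers itself with the inventory, configures lifebar and movement through BPCharStats, binds to status updates and pushes initial HP and EP.
; Tick polls the instigator controller through BPI_Controls to set jump and crouch flags.
; HP, EP, shooting-drain and stats-update functions are placeholder stubs, with the checks returning false.
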(event EventBeginPlay
  (bind _bp_char_stats (Variables|Default|GetBP_Char_Stats))
  (Variables|/Game/Blueprints/Player/Inventory.Inventory_C|SetSelfParent (Variables|Default|GetInventory) self)
  (Utilities|FlowControl|Sequence
    (:then_0
      (bind _lifebare (Default|ConfigLifebar (Variables|Default|GetBP_Char_Stats)))
      (Development|PrintString _lifebare true true "(R=0.000000,G=0.660000,B=1.000000,A=1.000000)" 6e+01))
    (:then_1
      (Default|ConfigMove (Variables|Default|GetBP_Char_Stats)))
    (:then_2
      (EventDispatchers|BindEventtoOnStatusUpdate (Variables|Default|GetBP_Char_Stats) (EventDispatchers|CreateEvent :!event BPonStatsUpdated))
      (CallFunction|OnStatsUpdated self false false (Variables|/Game/Blueprints/Companent/BP_Char_Stats.BP_Char_Stats_C|GetCurrentHP _bp_char_stats) (Variables|/Game/Blueprints/Companent/BP_Char_Stats.BP_Char_Stats_C|GetCurrentEP _bp_char_stats)))))

(event EventTick
  (params (DeltaSeconds :type Float%20%28single-precision%29))
  (CallFunction|CrouchandJump))

(fn ConstructionScript)

(fn CrouchandJump
  (bind _returnvalue (Game|GetInstigatorController))
  (if (Utilities|DoesObjectImplementInterface _returnvalue "/Game/Blueprints/Base/BPI_Controls.BPI_Controls_C")
    (bind (_outjump _outcrouch) (Class|BPIControls|WalkJumpCrouch(Message) _returnvalue))
    (Variables|Default|SetCharJump _outjump)
    (Variables|Default|SetCharCrouch _outcrouch)))

(fn BPonStatsUpdated
  (params (IsDead :type Boolean) (ItsDamage :type Boolean) (CurrentHP :type Integer) (CurrentEP :type Integer))
  (if IsDead
    _))

(fn CheckEP
  (return false))

(fn CheckHP
  (return false))

(fn SelfRef
  (return self))

(fn ShootingEnergyDrain
  (params (EnergyCost :type Integer))
  (return false))
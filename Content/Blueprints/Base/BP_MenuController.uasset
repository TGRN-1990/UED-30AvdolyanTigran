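; Menu player controller that creates the start and load menu widgets on BeginPlay, then shows the start menu.
; WInit adds both widgets hidden to the viewport and hands each a reference back to the controller.
; FlipFlop events toggle the start menu or swap it with the load menu.
; GamePause inverts StMenu, also the start widget's init flag, to set pause, feeding that call's return value into cursor and mouse-event settings.
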(event Custom|StartMenu
  (Utilities|FlowControl|FlipFlop
    (:A
      (CallFunction|GamePause (Variables|Default|GetS-Menu) (Variables|Default|GetVisable)))
    (:B
      (CallFunction|GamePause (Variables|Default|GetS-Menu) (Variables|Default|GetHidden)))))

(event Custom|LoadStartMenu
  (Utilities|FlowControl|FlipFlop
    (:A
      (CallFunction|VisibleSwap (Variables|Default|GetSL-Menu) (Variables|Default|GetS-Menu)))
    (:B
      (CallFunction|VisibleSwap (Variables|Default|GetS-Menu) (Variables|Default|GetSL-Menu)))))

(event EventBeginPlay
  (CallFunction|WInit)
  (CallFunction|StartMenu))

(event EventTick
  (params (DeltaSeconds :type Float%20%28single-precision%29)))

(fn ConstructionScript)

(fn WInit
  (Utilities|FlowControl|Sequence
    (:then_0
      (if (not (Variables|Default|GetStMenu))
        (bind _object (CallFunction|WidgetIni "/Game/Blueprints/BP_HUD/BP_Widjet/BP_Widjet_StartMenu.BP_Widjet_StartMenu_C"))
        (bind _asbp_widjet_start_menu (Utilities|Casting|CastToBP_Widjet_StartMenu _object))
        (bind _output_get (Variables|Default|SetS-Menu _asbp_widjet_start_menu))
        (Variables|/Game/Blueprints/BP_HUD/BP_Widjet/BP_Widjet_StartMenu.BP_Widjet_StartMenu_C|SetTargetControl _output_get self)
        (Variables|Default|SetStMenu true)))
    (:then_1
      (if (not (Variables|Default|GetStLMenu))
        (bind _object_2 (CallFunction|WidgetIni "/Game/Blueprints/BP_HUD/BP_Widjet/BP_Widjet_StartLoadMenu.BP_Widjet_StartLoadMenu_C"))
        (bind _asbp_widjet_start_load_menu (Utilities|Casting|CastToBP_Widjet_StartLoadMenu _object_2))
        (bind _output_get_2 (Variables|Default|SetSL-Menu _asbp_widjet_start_load_menu))
        (Variables|/Game/Blueprints/BP_HUD/BP_Widjet/BP_Widjet_StartLoadMenu.BP_Widjet_StartLoadMenu_C|SetTargetControl _output_get_2 self)
        (Variables|Default|SetStLMenu true)))))

(fn WidgetIni
  (params (Class :type User%20Widget%20Class%20Reference))
  (bind _returnvalue (UserInterface|CreateWidget Class))
  (UserInterface|Viewport|AddtoViewport _returnvalue 0)
  (Widget|SetVisibility _returnvalue "Hidden")
  (return _returnvalue))

(fn VisibleSwap
  (params (Vis :type User%20Widget%20Object%20Reference) (Hide :type User%20Widget%20Object%20Reference))
  (Widget|SetVisibility Vis "Visible")
  (Widget|SetVisibility Hide "Hidden"))

(fn GamePause
  (params (VisTarget :type User%20Widget%20Object%20Reference) (VisCount :type ESlateVisibility%20Enum :default "Visible"))
  (Widget|SetVisibility VisTarget VisCount)
  (bind _output_get (Variables|Default|SetStMenu (not (Variables|Default|GetStMenu))))
  (bind _returnvalue (Game|SetGamePaused _output_get))
  (bind _output_get_2 (Variables|Default|SetbShowMouseCursor _returnvalue))
  (bind _output_get_3 (Variables|Default|SetbEnableClickEvents _output_get_2))
  (Variables|Default|SetbEnableMouseOverEvents _output_get_3))
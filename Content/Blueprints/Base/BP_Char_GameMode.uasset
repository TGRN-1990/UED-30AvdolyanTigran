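; Game Mode that runs the save system: manual slots, fast save/load, checkpoints and level-transition saves.
; BP_Save slots, created on demand, store level, position, HP, EP and arsenal exchanged with BP_CharPlayer.
; Before loads or transitions, data is copied to a temporary slot and a BP_SaveManage flag is persisted.
; NextLevelLoad later reads that flag to restore full state, or only character stats after level transitions, then clears it.
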(event Custom|Inital
  ;[1 1 1] Инициализация слотов
  (Utilities|FlowControl|Sequence
    (:then_0
      (bind _returnvalue (CallFunction|CreateSlot (Variables|Default|GetSlotName1)))
      (Variables|Default|SetSlotSave1 _returnvalue))
    (:then_1
      (bind _returnvalue_2 (CallFunction|CreateSlot (Variables|Default|GetSlotName2)))
      (Variables|Default|SetSlotSave2 _returnvalue_2))
    (:then_2
      (bind _returnvalue_3 (CallFunction|CreateSlot (Variables|Default|GetSlotName3)))
      (Variables|Default|SetSlotSave3 _returnvalue_3))
    (:then_3
      (bind _returnvalue_4 (CallFunction|CreateSlot (Variables|Default|GetChekPoint)))
      (Variables|Default|SetCheckPointSlot _returnvalue_4))
    (:then_4
      (bind _returnvalue_5 (CallFunction|CreateSlot (Variables|Default|GetTempleSlotName)))
      (Variables|Default|SetTempleSlot _returnvalue_5))
    (:then_5
      (bind _returnvalue_6 (CallFunction|CreateSlot (Variables|Default|GetNextLevelSlotName)))
      (Variables|Default|SetNextLevelSlot _returnvalue_6))
    (:then_6
      (bind _returnvalue_7 (CallFunction|CreateSlot (Variables|Default|GetFastLoadName)))
      (Variables|Default|SetFastLoad _returnvalue_7))
    (:then_7
      (bind _returnvalue_8 (CallFunction|CreateManageSlot "1"))
      (Variables|Default|SetPre/PostLoad _returnvalue_8))
    (:then_8
      (bind _returnvalue_9 (CallFunction|CreateManageSlot "2"))
      (Variables|Default|SetSystemMenuIndication _returnvalue_9))))

(event Custom|CheckPoint%20Save
  (params (Lock :type Vector) (Tranlocation :type Transform))
  ;[1 1 1] Система Сохранения
  (CallFunction|Inital)
  (CallFunction|SaveSlotCheckPoints (Variables|Default|GetCheckPointSlot) (Variables|Default|GetChekPoint) Lock Tranlocation))

(event Custom|LoadSL2
  (bind _slotsave2 (Variables|Default|GetSlotSave2))
  (bind _slotname2 (Variables|Default|GetSlotName2))
  ;[1 1 1] Загрузка со слотов
  (CallFunction|Inital)
  (CallFunction|Pre-Post-LoadFormer (Variables|Default|GetPre/PostLoad) _slotsave2 _slotname2 (Variables|Default|GetTempleSlot) (Variables|Default|GetTempleSlotName))
  (CallFunction|LoadSlotFunLevel _slotsave2 _slotname2))

(event Custom|Next%20level
  ;[1 1 1] До-загрузка перехода на уровень
  (CallFunction|Inital)
  (CallFunction|LoadSlotFunChar (Variables|Default|GetTempleSlot) (Variables|Default|GetTempleSlotName))
  (CallFunction|FLSave))

(event Custom|Next%20level%20Save
  ;[1 1 1] Система Сохранения
  (CallFunction|Inital)
  (CallFunction|SaveSlotFun (Variables|Default|GetNextLevelSlot) (Variables|Default|GetNextLevelSlotName))
  (CallFunction|NextLevelFormer (Variables|Default|GetPre/PostLoad) (Variables|Default|GetNextLevelSlot) (Variables|Default|GetNextLevelSlotName) (Variables|Default|GetTempleSlot) (Variables|Default|GetTempleSlotName)))

(event Custom|LoadSL3
  (bind _slotname3 (Variables|Default|GetSlotName3))
  (bind _slotsave3 (Variables|Default|GetSlotSave3))
  ;[1 1 1] Загрузка со слотов
  (CallFunction|Inital)
  (CallFunction|Pre-Post-LoadFormer (Variables|Default|GetPre/PostLoad) _slotsave3 _slotname3 (Variables|Default|GetTempleSlot) (Variables|Default|GetTempleSlotName))
  (CallFunction|LoadSlotFunLevel _slotsave3 _slotname3))

(event Custom|CheckPointLoad
  (bind _chekpoint (Variables|Default|GetChekPoint))
  (bind _checkpointslot (Variables|Default|GetCheckPointSlot))
  ;[1 1 1] Чекпоинты - загрузка на уровне после смерти/
  (CallFunction|Inital)
  (CallFunction|LoadSlotFunChar _checkpointslot _chekpoint)
  (CallFunction|LoadSlotFunCoordinate _checkpointslot _chekpoint))

(event Custom|SaveSL3
  ;[1 1 1] Система Сохранения
  (CallFunction|Inital)
  (CallFunction|SaveSlotFun (Variables|Default|GetSlotSave3) (Variables|Default|GetSlotName3)))

(event Custom|SaveSL1
  ;[1 1 1] Система Сохранения
  (CallFunction|Inital)
  (CallFunction|SaveSlotFun (Variables|Default|GetSlotSave1) (Variables|Default|GetSlotName1)))

(event Custom|FL_Slot_Load
  (bind _fastloadname (Variables|Default|GetFastLoadName))
  (bind _fastload (Variables|Default|GetFastLoad))
  ;[1 1 1] Загрузка со слотов
  (CallFunction|Inital)
  (CallFunction|Pre-Post-LoadFormer (Variables|Default|GetPre/PostLoad) _fastload _fastloadname (Variables|Default|GetTempleSlot) (Variables|Default|GetTempleSlotName))
  (CallFunction|LoadSlotFunLevel _fastload _fastloadname))

(event Custom|SaveSL2
  ;[1 1 1] Система Сохранения
  (CallFunction|Inital)
  (CallFunction|SaveSlotFun (Variables|Default|GetSlotSave2) (Variables|Default|GetSlotName2)))

(event Custom|PrePostLoad
  (bind _templeslot (Variables|Default|GetTempleSlot))
  (bind _templeslotname (Variables|Default|GetTempleSlotName))
  ;[1 1 1] До-загрузка после загрузки уровня
  (CallFunction|Inital)
  (CallFunction|LoadSlotFunChar _templeslot _templeslotname)
  (CallFunction|LoadSlotFunCoordinate _templeslot _templeslotname))

(event Custom|LoadSL1
  (bind _slotsave1 (Variables|Default|GetSlotSave1))
  (bind _slotname1 (Variables|Default|GetSlotName1))
  ;[1 1 1] Загрузка со слотов
  (CallFunction|Inital)
  (CallFunction|Pre-Post-LoadFormer (Variables|Default|GetPre/PostLoad) _slotsave1 _slotname1 (Variables|Default|GetTempleSlot) (Variables|Default|GetTempleSlotName))
  (CallFunction|LoadSlotFunLevel _slotsave1 _slotname1))

(event Custom|FL_save
  ;[1 1 1] Система Сохранения
  (CallFunction|Inital)
  (CallFunction|SaveSlotFun (Variables|Default|GetFastLoad) (Variables|Default|GetFastLoadName)))

(event EventBeginPlay
  ;[1 1 1] Инициализация слотов
  (Utilities|FlowControl|Sequence
    (:then_0
      (bind _returnvalue (CallFunction|CreateSlot (Variables|Default|GetSlotName1)))
      (Variables|Default|SetSlotSave1 _returnvalue))
    (:then_1
      (bind _returnvalue_2 (CallFunction|CreateSlot (Variables|Default|GetSlotName2)))
      (Variables|Default|SetSlotSave2 _returnvalue_2))
    (:then_2
      (bind _returnvalue_3 (CallFunction|CreateSlot (Variables|Default|GetSlotName3)))
      (Variables|Default|SetSlotSave3 _returnvalue_3))
    (:then_3
      (bind _returnvalue_4 (CallFunction|CreateSlot (Variables|Default|GetChekPoint)))
      (Variables|Default|SetCheckPointSlot _returnvalue_4))
    (:then_4
      (bind _returnvalue_5 (CallFunction|CreateSlot (Variables|Default|GetTempleSlotName)))
      (Variables|Default|SetTempleSlot _returnvalue_5))
    (:then_5
      (bind _returnvalue_6 (CallFunction|CreateSlot (Variables|Default|GetNextLevelSlotName)))
      (Variables|Default|SetNextLevelSlot _returnvalue_6))
    (:then_6
      (bind _returnvalue_7 (CallFunction|CreateSlot (Variables|Default|GetFastLoadName)))
      (Variables|Default|SetFastLoad _returnvalue_7))
    (:then_7
      (bind _returnvalue_8 (CallFunction|CreateManageSlot "1"))
      (Variables|Default|SetPre/PostLoad _returnvalue_8))
    (:then_8
      (bind _returnvalue_9 (CallFunction|CreateManageSlot "2"))
      (Variables|Default|SetSystemMenuIndication _returnvalue_9))))

(fn ConstructionScript)

(fn CreateSlot
  (params (SlotName :type String))
  (bind _output_get (LocalVariables|SetInitName SlotName))
  (bind _returnvalue (SaveGame|DoesSaveGameExist _output_get))
  (if _returnvalue
    _
    (else
      (bind _returnvalue_2 (SaveGame|CreateSaveGameObject "/Game/Blueprints/Save/BP_Save.BP_Save_C"))
      (SaveGame|SaveGametoSlot _returnvalue_2 (LocalVariables|GetInitName))))
  (bind _returnvalue_3 (SaveGame|LoadGamefromSlot (LocalVariables|GetInitName)))
  (bind _asbp_save (Utilities|Casting|CastToBP_Save _returnvalue_3))
  (bind _output_get_2 (LocalVariables|SetInitSlot _asbp_save))
  (return _output_get_2))

(fn SaveSlotFun
  (params (SaveSlot :type BP%20Save%20Object%20Reference) (SlotName :type String))
  (LocalVariables|SetSaveSlotName SlotName)
  (LocalVariables|SetSaveSaveSlot SaveSlot)
  (bind _asbp_char_player (Utilities|Casting|CastToBP_CharPlayer (Game|GetPlayerCharacter 0)))
  (bind (_levelname _playervector _playertransform _current_hp _current_ep _arsenal) (Default|CheckforSave _asbp_char_player _asbp_char_player))
  (bind _asbp_save (Utilities|Casting|CastToBP_Save (LocalVariables|GetSaveSaveSlot)))
  (Default|SaveInput _asbp_save _levelname _playervector _playertransform _current_hp _current_ep _arsenal)
  (SaveGame|SaveGametoSlot (LocalVariables|GetSaveSaveSlot) (LocalVariables|GetSaveSlotName))
  (return))

(fn LoadSlotFunLevel
  (params (Target%20Slot :type BP%20Save%20Object%20Reference) (SlotName :type String))
  (bind _output_get (LocalVariables|SetLoadSlotName SlotName))
  (LocalVariables|SetLoadSlotFun Target%20Slot)
  (bind _returnvalue (SaveGame|LoadGamefromSlot _output_get))
  (bind _asbp_save (Utilities|Casting|CastToBP_Save _returnvalue))
  (bind _level (Default|LoadOutput _asbp_save _asbp_save))
  (if (Utilities|Name|NotEqual(Name) _level "MainMenuLevel")
    (Game|OpenLevel(byName) _level)))

(fn LoadSlotFunChar
  (params (Target%20Slot :type BP%20Save%20Object%20Reference) (SlotName :type String))
  (bind _output_get (LocalVariables|SetLoadSlotName SlotName))
  (LocalVariables|SetLoadSlotFun Target%20Slot)
  (bind _returnvalue (SaveGame|LoadGamefromSlot _output_get))
  (bind _asbp_save (Utilities|Casting|CastToBP_Save _returnvalue))
  (bind (_level _hp _ep _arsenal) (Default|LoadOutput _asbp_save _asbp_save))
  (bind _asbp_char_player (Utilities|Casting|CastToBP_CharPlayer (Game|GetPlayerCharacter 0)))
  (Default|CheckforLoadChar _asbp_char_player _hp _ep _arsenal _asbp_char_player))

(fn LoadSlotFunCoordinate
  (params (Target%20Slot :type BP%20Save%20Object%20Reference) (SlotName :type String))
  (bind _output_get (LocalVariables|SetLoadSlotName SlotName))
  (LocalVariables|SetLoadSlotFun Target%20Slot)
  (bind _returnvalue (SaveGame|LoadGamefromSlot _output_get))
  (bind _asbp_save (Utilities|Casting|CastToBP_Save _returnvalue))
  (bind (_level _hp _ep _arsenal _lock _transform) (Default|LoadOutput _asbp_save _asbp_save))
  (bind _asbp_char_player (Utilities|Casting|CastToBP_CharPlayer (Game|GetPlayerCharacter 0)))
  (Default|CheckforLoadCoor _asbp_char_player _lock _transform _asbp_char_player))

(fn CreateManageSlot
  (params (SlotName :type String))
  (bind _returnvalue (SaveGame|DoesSaveGameExist SlotName))
  (if _returnvalue
    _
    (else
      (bind _returnvalue_2 (SaveGame|CreateSaveGameObject "/Game/Blueprints/Save/BP_SaveManage.BP_SaveManage_C"))
      (SaveGame|SaveGametoSlot _returnvalue_2 SlotName)))
  (bind _returnvalue_3 (SaveGame|LoadGamefromSlot SlotName))
  (bind _asbp_save_manage (Utilities|Casting|CastToBP_SaveManage _returnvalue_3))
  (bind _output_get (LocalVariables|SetInitSlot _asbp_save_manage))
  (return _output_get))

(fn Pre-Post-LoadFormer
  (params (Manage :type BP%20Save%20Manage%20Object%20Reference) (Slot :type BP%20Save%20Object%20Reference) (SlotName :type String) (TempleSlot :type BP%20Save%20Object%20Reference) (TempleNameSlot :type String))
  ;[1 1 1] Якорь для дозагрузки
  (bind _asbp_save_manage (Utilities|Casting|CastToBP_SaveManage Manage))
  (Variables|/Game/Blueprints/Save/BP_SaveManage.BP_SaveManage_C|SetLoad-Post-Load _asbp_save_manage true)
  (SaveGame|SaveGametoSlot _asbp_save_manage "1")
  ;[1 1 1] Резервное сохранение для дозагрузки
  (Utilities|Casting|CastToBP_Save Slot)
  (bind _returnvalue (SaveGame|LoadGamefromSlot SlotName))
  (bind _asbp_save (Utilities|Casting|CastToBP_Save _returnvalue))
  (bind (_level _hp _ep _arsenal _lock _transform) (Default|LoadOutput _asbp_save _asbp_save))
  (if (Utilities|Name|NotEqual(Name) _level "MainMenuLevel")
    (bind _asbp_save_2 (Utilities|Casting|CastToBP_Save TempleSlot))
    (Default|SaveInput _asbp_save_2 (Utilities|String|ToString(Name) _level) _lock _transform _hp _ep _arsenal)
    (SaveGame|SaveGametoSlot _asbp_save_2 TempleNameSlot)
    (return)))

(fn Save-to-Save
  (params (SaveSlot :type BP%20Save%20Object%20Reference) (SlotName :type String))
  (LocalVariables|SetSaveSlotName SlotName)
  (LocalVariables|SetSaveSaveSlot SaveSlot)
  (bind _asbp_char_player (Utilities|Casting|CastToBP_CharPlayer (Game|GetPlayerCharacter 0)))
  (bind (_levelname _playervector _playertransform _current_hp _current_ep _arsenal) (Default|CheckforSave _asbp_char_player _asbp_char_player))
  (bind _asbp_save (Utilities|Casting|CastToBP_Save (LocalVariables|GetSaveSaveSlot)))
  (Default|SaveInput _asbp_save _levelname _playervector _playertransform _current_hp _current_ep _arsenal)
  (SaveGame|SaveGametoSlot (LocalVariables|GetSaveSaveSlot) (LocalVariables|GetSaveSlotName))
  (return (LocalVariables|GetSaveSaveSlot)))

(fn MenuVisible
  (bind _asbp_char_controlls (Utilities|Casting|CastToBP_CharControlls (Game|GetPlayerController 0)))
  (Default|WidjetInit _asbp_char_controlls)
  (bind _asbp_char_player (Utilities|Casting|CastToBP_CharPlayer (Game|Player|GetPlayerPawn 0)))
  (Rendering|SetVisibility (Variables|/Game/Blueprints/Player/BP_CharPlayer.BP_CharPlayer_C|GetWidgetChar _asbp_char_player) true false))

(fn NextLevelLoad
  (SaveGame|LoadGamefromSlot "1")
  (bind _asbp_save_manage (Utilities|Casting|CastToBP_SaveManage (Variables|Default|GetPre/PostLoad)))
  (if (Variables|/Game/Blueprints/Save/BP_SaveManage.BP_SaveManage_C|GetLoad-From-Level _asbp_save_manage)
    (CallFunction|NextLevel)
    (bind _asbp_save_manage_2 (Utilities|Casting|CastToBP_SaveManage (Variables|Default|GetPre/PostLoad)))
    (Variables|/Game/Blueprints/Save/BP_SaveManage.BP_SaveManage_C|SetLoad-From-Level _asbp_save_manage_2 false)
    (SaveGame|SaveGametoSlot _asbp_save_manage_2 "1")
    (elif (Variables|/Game/Blueprints/Save/BP_SaveManage.BP_SaveManage_C|GetLoad-Post-Load _asbp_save_manage)
      (CallFunction|PrePostLoad)
      (bind _asbp_save_manage_3 (Utilities|Casting|CastToBP_SaveManage (Variables|Default|GetPre/PostLoad)))
      (Variables|/Game/Blueprints/Save/BP_SaveManage.BP_SaveManage_C|SetLoad-Post-Load _asbp_save_manage_3 false)
      (SaveGame|SaveGametoSlot _asbp_save_manage_3 "1"))))

(fn NextLevelFormer
  (params (Manage :type BP%20Save%20Manage%20Object%20Reference) (Slot :type BP%20Save%20Object%20Reference) (SlotName :type String) (TempleSlot :type BP%20Save%20Object%20Reference) (TempleNameSlot :type String))
  ;[1 1 1] Якорь для дозагрузки
  (bind _asbp_save_manage (Utilities|Casting|CastToBP_SaveManage Manage))
  (Variables|/Game/Blueprints/Save/BP_SaveManage.BP_SaveManage_C|SetLoad-From-Level _asbp_save_manage true)
  (SaveGame|SaveGametoSlot _asbp_save_manage "1")
  ;[1 1 1] Резервное сохранение для дозагрузки
  (Utilities|Casting|CastToBP_Save Slot)
  (bind _returnvalue (SaveGame|LoadGamefromSlot SlotName))
  (bind _asbp_save (Utilities|Casting|CastToBP_Save _returnvalue))
  (bind (_level _hp _ep _arsenal _lock _transform) (Default|LoadOutput _asbp_save _asbp_save))
  (bind _asbp_save_2 (Utilities|Casting|CastToBP_Save TempleSlot))
  (Default|SaveInput _asbp_save_2 "" _lock _transform _hp _ep _arsenal)
  (SaveGame|SaveGametoSlot _asbp_save_2 TempleNameSlot)
  (return))

(fn StartFixLoad
  (bind _returnvalue (SaveGame|LoadGamefromSlot "2"))
  (bind _asbp_save_manage (Utilities|Casting|CastToBP_SaveManage _returnvalue))
  (Variables|Default|SetGameStart (Variables|/Game/Blueprints/Save/BP_SaveManage.BP_SaveManage_C|GetFixLevel _asbp_save_manage)))

(fn FixSave
  (params (InputPin :type Boolean))
  (bind _asbp_char_game_mode (Utilities|Casting|CastToBP_Char_GameMode (Game|GetGameMode)))
  (bind _asbp_save_manage (Utilities|Casting|CastToBP_SaveManage (Variables|BP_Char_GameMode_C|GetSystemMenuIndication _asbp_char_game_mode)))
  (Variables|/Game/Blueprints/Save/BP_SaveManage.BP_SaveManage_C|SetFixLevel _asbp_save_manage InputPin)
  (SaveGame|SaveGametoSlot _asbp_save_manage "2"))

(fn SaveSlotCheckPoints
  (params (SaveSlot :type BP%20Save%20Object%20Reference) (SlotName :type String) (CheckLock :type Vector) (CheckTranslocation :type Transform))
  (LocalVariables|SetSaveSlotName SlotName)
  (LocalVariables|SetSaveSaveSlot SaveSlot)
  (bind _asbp_char_player (Utilities|Casting|CastToBP_CharPlayer (Game|GetPlayerCharacter 0)))
  (bind (_levelname _playervector _playertransform _current_hp _current_ep _arsenal) (Default|CheckforSave _asbp_char_player _asbp_char_player))
  (bind _asbp_save (Utilities|Casting|CastToBP_Save (LocalVariables|GetSaveSaveSlot)))
  (Default|SaveInput _asbp_save _levelname CheckLock CheckTranslocation _current_hp _current_ep _arsenal)
  (SaveGame|SaveGametoSlot (LocalVariables|GetSaveSaveSlot) (LocalVariables|GetSaveSlotName))
  (return))